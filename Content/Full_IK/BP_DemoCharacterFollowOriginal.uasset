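; Demo character Blueprint that supplies full-body IK effectors that follow the original animated foot location and rotation.
; GetEffectors builds one effector per foot, rooted at the pelvis, using the relative Z of the FootingL and FootingR components as the Z location.
; An OffsetTL timeline is set up to move both footing components vertically, but nothing starts it in this graph.
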(fn `GetEffectors`
  (returns (Effectors :type "Array of AnimNode_FullbodyIkEffector Structure"))
  (locals (Effectors_ :type "Array of AnimNode_FullbodyIkEffector Structure"))
  (bind (_relativelocation_x _relativelocation_y _relativelocation_z) (`KismetMathLibrary.BreakVector` (`SceneComponent.RelativeLocation` (`self.FootingR`))))
  (bind (_relativelocation_x_2 _relativelocation_y_2 _relativelocation_z_2) (`KismetMathLibrary.BreakVector` (`SceneComponent.RelativeLocation` (`self.FootingL`))))
  (`|ExecutionSequence`
    (:`then_0`
      (`|ExecutionSequence`
        (:`then_0`
          (`KismetArrayLibrary.Array_Add` (`local.Effectors_`) (make `AnimNode_FullbodyIkEffector` "FollowOriginalLocationAndRotation" "foot_l" "pelvis" (`KismetMathLibrary.MakeVector` 0.0 0.0 _relativelocation_z_2))))
        (:`then_1`
          (`KismetArrayLibrary.Array_Add` (`local.Effectors_`) (make `AnimNode_FullbodyIkEffector` "FollowOriginalLocationAndRotation" "foot_r" "pelvis" (`KismetMathLibrary.MakeVector` 0.0 0.0 _relativelocation_z))))))
    (:`then_1`
      (return (`local.Effectors_`)))))

(fn `UserConstructionScript`
  (`parent.UserConstructionScript`))