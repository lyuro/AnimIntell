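; Demo character for Full-Body IK that pins hands, feet and head to target actors using Keep-type effectors.
; GetEffectors adds an effector for each valid target: hands keep location at the middle finger bones, while feet and head keep location and rotation.
; MakeEffector holds a node that builds an IK effector from the target actor's transform with pelvis as root bone.
; Event graph and construction script add no logic.
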(fn `GetEffectors`
  (returns (Effectors :type "Array of AnimNode_FullbodyIkEffector Structure"))
  (locals (Effectors_ :type "Array of AnimNode_FullbodyIkEffector Structure"))
  (`|ExecutionSequence`
    (:`then_0`
      (`|ExecutionSequence`
        (:`then_0`
          (bind _handl (`self.HandL`)
            (:`then`
              (`KismetArrayLibrary.Array_Add` (`local.Effectors_`) (`self.MakeEffector` "KeepLocation" "middle_01_l" _handl)))
            (:`else`)))
        (:`then_1`
          (bind _handr (`self.HandR`)
            (:`then`
              (`KismetArrayLibrary.Array_Add` (`local.Effectors_`) (`self.MakeEffector` "KeepLocation" "middle_01_r" _handr)))
            (:`else`)))
        (:`then_2`
          (bind _footl (`self.FootL`)
            (:`then`
              (`KismetArrayLibrary.Array_Add` (`local.Effectors_`) (`self.MakeEffector` "KeepLocationAndRotation" "foot_l" _footl)))
            (:`else`)))
        (:`then_3`
          (bind _footr (`self.FootR`)
            (:`then`
              (`KismetArrayLibrary.Array_Add` (`local.Effectors_`) (`self.MakeEffector` "KeepLocationAndRotation" "foot_r" _footr)))
            (:`else`)))
        (:`then_4`
          (bind _head (`self.Head`)
            (:`then`
              (`KismetArrayLibrary.Array_Add` (`local.Effectors_`) (`self.MakeEffector` "KeepLocationAndRotation" "head" _head)))
            (:`else`)))))
    (:`then_1`
      (return (`local.Effectors_`)))))

(fn `UserConstructionScript`
  (`parent.UserConstructionScript`))